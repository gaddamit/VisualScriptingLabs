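; BP_Lever is a lever actor that activates one or more attached BP_Elevator actors.
; On BeginPlay it attaches the nearest elevator in the level if none are assigned.
; Activate proceeds only when no attached elevator is moving, then calls each elevator.
; Inside that same loop, MoveComponentTo rotates the lever between original and target orientations and flips IsLeverDown, so the toggle repeats per elevator.
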(event Custom|Activate
  (bind _value (CallFunction|AreAllElevatorsStopped))
  (if _value
    (|ActivateAttachedElevator)))

(event EventBeginPlay
  (if (== (Utilities|Array|Length (Variables|Default|GetElevator)) 0)
    (CallFunction|FindandAttachNearestElevator)))

(fn ConstructionScript)

(fn AreAllElevatorsStopped
  (for _array_element (Variables|Default|GetElevator)
    (if (Variables|/Game/Blueprints/BP_Elevator.BP_Elevator_C|GetIsMoving _array_element)
      (return false)))
  (return true))

(fn FindandAttachNearestElevator
  (bind _outactors (Actor|GetAllActorsOfClass "/Game/Blueprints/BP_Elevator.BP_Elevator_C"))
  (bind _asbp_elevator (Utilities|Casting|CastToBP_Elevator (.ReturnValue (Actor|FindNearestActor (Transformation|GetWorldLocation (Variables|Default|GetDefaultSceneRoot)) _outactors))))
  (Utilities|Array|Add (Variables|Default|GetElevator) _asbp_elevator))