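; A sliding door that opens when the third-person character enters its collision volume and closes when they leave, showing a greeting message once open.
; MoveComponentTo eases the door between its original and target positions, and an IsSliding flag ignores requests made mid-slide.
; An optional PartnerDoor is driven through force open and close events that skip re-notifying the partner.
; The construction script sets the greeting text and optionally re-orients it.
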(event OnComponentBeginOverlap(CollisionVolume)
  (params (OverlappedComponent :type Primitive%20Component%20Object%20Reference) (OtherActor :type Actor%20Object%20Reference) (OtherComp :type Primitive%20Component%20Object%20Reference) (OtherBodyIndex :type Integer) (bFromSweep :type Boolean) (SweepResult :type Hit%20Result%20Structure%20%28by%20ref%29))
  (Utilities|Casting|CastToBP_ThirdPersonCharacter OtherActor)
  (Utilities|IsValid (Variables|Door|GetPartnerDoor)
    (:Is%20Valid
      (CallFunction|ForceOpenDoor (Variables|Door|GetPartnerDoor)))
    (:Is%20Not%20Valid
      _))
  (if (not (Variables|Door|GetIsSliding))
    (Variables|Door|SetIsSliding true)
    (Components|MoveComponentTo (Variables|Default|GetDoor) (Variables|Position|GetPositionTarget) "0, 0, 0" true true (Variables|Door|GetSlideTime) false)
    (Variables|Door|SetIsSliding false)
    (Development|SetHiddeninGame (Variables|Default|GetMessage) false false)))

(event OnComponentEndOverlap(CollisionVolume)
  (params (OverlappedComponent :type Primitive%20Component%20Object%20Reference) (OtherActor :type Actor%20Object%20Reference) (OtherComp :type Primitive%20Component%20Object%20Reference) (OtherBodyIndex :type Integer))
  (Utilities|Casting|CastToBP_ThirdPersonCharacter OtherActor)
  (Utilities|IsValid (Variables|Door|GetPartnerDoor)
    (:Is%20Valid
      (CallFunction|ForceCloseDoor (Variables|Door|GetPartnerDoor)))
    (:Is%20Not%20Valid
      _))
  (if (not (Variables|Door|GetIsSliding))
    (Variables|Door|SetIsSliding true)
    (Components|MoveComponentTo (Variables|Default|GetDoor) (Variables|Position|GetPositionOriginal) "0, 0, 0" true true (Variables|Door|GetSlideTime) false)
    (Variables|Door|SetIsSliding false)
    (Development|SetHiddeninGame (Variables|Default|GetMessage) true false)))

(event Custom|ForceCloseDoor
  (if (not (Variables|Door|GetIsSliding))
    (Variables|Door|SetIsSliding true)
    (Components|MoveComponentTo (Variables|Default|GetDoor) (Variables|Position|GetPositionOriginal) "0, 0, 0" true true (Variables|Door|GetSlideTime) false)
    (Variables|Door|SetIsSliding false)
    (Development|SetHiddeninGame (Variables|Default|GetMessage) true false)))

(event Custom|ForceOpenDoor
  (if (not (Variables|Door|GetIsSliding))
    (Variables|Door|SetIsSliding true)
    (Components|MoveComponentTo (Variables|Default|GetDoor) (Variables|Position|GetPositionTarget) "0, 0, 0" true true (Variables|Door|GetSlideTime) false)
    (Variables|Door|SetIsSliding false)
    (Development|SetHiddeninGame (Variables|Default|GetMessage) false false)))

(event EventBeginPlay
  (Variables|Position|SetPositionOriginal (Variables|/Script/Engine.SceneComponent|GetRelativeLocation (Variables|Default|GetDoor)))
  (Variables|Position|SetPositionTarget (Variables|Position|GetPositionTarget))
  (Development|SetHiddeninGame (Variables|Default|GetMessage) true false))

(fn ConstructionScript
  (bind _message (Variables|Default|GetMessage))
  (Rendering|Components|TextRender|SetText (Variables|Default|GetMessage) (Utilities|Text|ToText(String) (Variables|DisplayText|GetGreetingText)))
  (if (Variables|DisplayText|GetFlipText)
    (Rendering|Components|TextRender|SetHorizontalAlignment _message "EHTA_Center")
    (Transformation|SetRelativeRotation _message "0, 0, 0" false false)))