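; BP_Sphere is a sphere actor that takes a random color and gets knocked away when hit by a trace.
; The construction script creates a dynamic material from the red basic shape material and randomizes its Color parameter.
; The OnTrace override calls the parent, applies an impulse at the hit location along the source's forward vector, prints its name, and sets a lifespan for delayed destruction.
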(event EventBeginPlay)

(event Collision|EventActorBeginOverlap
  (params (OtherActor :type Actor%20Object%20Reference)))

(event EventTick
  (params (DeltaSeconds :type Float%20%28single-precision%29)))

(fn ConstructionScript
  (|CallParentFunction)
  (bind _returnvalue (Rendering|Material|CreateDynamicMaterialInstance (Variables|Default|GetSphere) 0 "/Game/Materials/M_BasicShapeMaterial_Red.M_BasicShapeMaterial_Red" "None" :!class /Script/Engine.PrimitiveComponent))
  (Rendering|Material|SetVectorParameterValue _returnvalue "Color" (Math|Color|MakeColor (Math|Random|RandomFloat) (Math|Random|RandomFloat) (Math|Random|RandomFloat)) :!class /Script/Engine.MaterialInstanceDynamic))

(fn OnTrace
  (params (Location :type Vector :default "0, 0, 0") (Source :type Actor%20Object%20Reference))
  (|CallParentFunction Location Source)
  (Physics|AddImpulseatLocation (Variables|Default|GetSphere) (* (Transformation|GetActorForwardVector Source) (Variables|Default|GetImpulseMultiplier)) Location "None")
  (Development|PrintString (Utilities|GetDisplayName self))
  (Actor|SetLifeSpan (Variables|Default|GetLifeSpanOnHit)))