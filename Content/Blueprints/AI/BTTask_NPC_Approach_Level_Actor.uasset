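; Behavior Tree task that sends the NPC to a randomly chosen Character in the level and interacts with it.
; AI MoveTo approaches the target, then calls Interact through BPI_InteractableActor.
; The self check compares a separate random pick against the task, not the controlled pawn.
; A failed move fails the task, while a target lacking the interface leaves it unfinished.
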(event EventReceiveExecuteAI
  (params (OwnerController :type AI%20Controller%20Object%20Reference) (ControlledPawn :type Pawn%20Object%20Reference))
  (bind _outactors (Actor|GetAllActorsOfClass "/Script/Engine.Character"))
  (Variables|Default|SetTargetActor (.OutItem (Utilities|Array|Random _outactors)))
  (if (== (.OutItem (Utilities|Array|Random _outactors)) self)
    (AI|BehaviorTree|FinishExecute false)
    (else
      (AI|AIMoveTo ControlledPawn (Transformation|GetActorLocation (Variables|Default|GetTargetActor)) (Variables|Default|GetTargetActor) (Variables|Default|GetAcceptance%20Radius) false
        (:OnSuccess
          (bind _asbpi_interactable_actor (Utilities|Casting|CastToBPI_InteractableActor (Variables|Default|GetTargetActor)))
          (Default|Interact _asbpi_interactable_actor)
          (AI|BehaviorTree|FinishExecute true))
        (:OnFail
          (AI|BehaviorTree|FinishExecute false))))))