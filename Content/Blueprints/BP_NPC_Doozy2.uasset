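; BP_NPC_Doozy2 is a Doozy character that takes key input to carry items and progress through the PuzzleBoss levels.
; E box-traces for physics items and attaches them to the head through a physics constraint, or drops them; in Level4 it triggers sleep and a music change instead.
; Qualifying mesh overlaps fade out and open the next numbered level, wrapping after the last.
; Destruction before finishing reloads the level, and Q toggles a cheat flag.
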(event OnComponentBeginOverlap(Mesh)
  (params (OverlappedComponent :type Primitive%20Component%20Object%20Reference) (OtherActor :type Actor%20Object%20Reference) (OtherComp :type Primitive%20Component%20Object%20Reference) (OtherBodyIndex :type Integer) (bFromSweep :type Boolean) (SweepResult :type Hit%20Result%20Structure%20%28by%20ref%29))
  (Utilities|Casting|CastTo OtherActor
    (:then
      _)
    (:CastFailed
      (Utilities|Casting|CastTo OtherActor)))
  (Variables|Default|SetIsLevelFinished true)
  (if (== (Variables|Default|GetCurrentLevel) (Variables|Default|GetMaxLevels))
    (Variables|Default|SetCurrentLevel 1)
    (else
      (Math|Integer|IncrementInt (Variables|Default|GetCurrentLevel)
        (:%20%20
          _))))
  (CameraFades|StartCameraFade :self (Game|GetPlayerCameraManager 0) :ToAlpha 1.0 :Duration 3.0 :bShouldFadeAudio true)
  (Pawn|Components|CharacterMovement|DisableMovement (Variables|Character|GetCharacterMovement))
  (Utilities|FlowControl|Delay 2.9)
  (Game|OpenLevel(byName) (Utilities|String|StringToName (Utilities|String|Append "PuzzleBoss_Level" (Utilities|String|ToString(Integer) (Variables|Default|GetCurrentLevel))))))

(event EventDestroyed
  (if (not (Variables|Default|GetIsLevelFinished))
    (Game|OpenLevel(byName) (Utilities|String|StringToName (Utilities|String|Append "PuzzleBoss_Level" (Utilities|String|ToString(Integer) (Variables|Default|GetCurrentLevel)))))))

(event EventBeginPlay
  (|CallParentFunction)
  (CameraFades|StartCameraFade :self (Game|GetPlayerCameraManager 0) :FromAlpha 1.0 :Duration 3.0))

(event Input|KeyboardEvents|E
  (params (Key :type Key%20Structure :default "None"))
  (bind _returnvalue (|CalculateBoxLocation))
  (bind _carryableitem (Variables|Carrying|GetCarryableItem))
  (:Pressed
    (bind _returnvalue_2 (Game|GetCurrentLevelName true))
    (if (Utilities|Enum|Equal(Enum) _returnvalue_2 "PuzzleBoss_Level4")
      (if (not (Variables|Default|GetIsSleeping))
        (if (Variables|Default|GetCanSleep)
          (Variables|Default|SetIsSleeping true)
          (Pawn|Components|CharacterMovement|DisableMovement (Variables|Character|GetCharacterMovement))
          (Default|CallChangeBackgroundMusic)))
      (elif (Variables|Carrying|GetIsCarrying)
        (Variables|Carrying|SetIsCarrying false)
        (Class|PhysicsConstraintComponent|BreakConstraint (Variables|Default|GetCarryItemAnchor)) ; Detach item from player
        (|DropCurrentItem)
        (else
          (bind (_outhit _returnvalue_3) (Class|KismetSystemLibrary|BoxTraceSingleforObjects _returnvalue _returnvalue "25.000000,25.000000,50.000000" (Transformation|GetActorRotation) (Utilities|Array|MakeArray "ObjectTypeQuery4") false 0 "None" true)) ; Check for items in front of player
          (if _returnvalue_3
            (bind _asbp_carryable_item (Utilities|Casting|CastTo (.HitActor (Collision|BreakHitResult _outhit))))
            (|CarryNewItem _asbp_carryable_item (.HitComponent (Collision|BreakHitResult _outhit)))
            (else
              (Variables|Carrying|SetIsCarrying false)
              (Utilities|IsValid _carryableitem
                (:Is%20Valid
                  (CallFunction|DropItem _carryableitem))))))))))

(event Input|KeyboardEvents|Q
  (params (Key :type Key%20Structure :default "None"))
  (:Pressed
    (bind _output_get (Variables|Default|SetEnableCheats (not (Variables|Default|GetEnableCheats))))
    (if _output_get
      (Development|PrintString "Cheat Enabled")
      (else
        (Development|PrintString "Cheat Disabled")))))

(fn ConstructionScript
  (|CallParentFunction))

(fn TryJump
  (if (Variables|Carrying|GetIsCarrying)
    _))

(fn CallRestartPlayer)